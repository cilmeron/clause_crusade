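; GingerBreadMaster is a gingerbread enemy character that roams, chases BP_Santa once pawn sensing spots a pawn, and attacks in melee.
; An overlap box toggles between chasing and timed attacks that drain Santa's health and load GameOver at zero.
; Delayed Tick logic re-triggers roaming, chasing or attacking.
; Damage adds to Santa's Highscore, with neck hits killing instantly as headshots, and death ragdolls the body before destroying it.
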(event OnSeePawn(PawnSensing)
  (params (Pawn :type Pawn%20Object%20Reference))
  (Variables|Default|Settarget Pawn)
  (Variables|Default|Setfirstfind true)
  (CallFunction|ChasePlayer))

(event OnComponentBeginOverlap(InRangeBox)
  (params (OverlappedComponent :type Primitive%20Component%20Object%20Reference) (OtherActor :type Actor%20Object%20Reference) (OtherComp :type Primitive%20Component%20Object%20Reference) (OtherBodyIndex :type Integer) (bFromSweep :type Boolean) (SweepResult :type Hit%20Result%20Structure%20%28by%20ref%29))
  (bind _asbp_santa (Utilities|Casting|CastToBP_Santa OtherActor))
  (Variables|Default|Settpc _asbp_santa)
  (Variables|Default|SetinRange true)
  (Components|Movement|StopMovementImmediately (Variables|Character|GetCharacterMovement))
  (CallFunction|Attacking))

(event OnComponentEndOverlap(InRangeBox)
  (params (OverlappedComponent :type Primitive%20Component%20Object%20Reference) (OtherActor :type Actor%20Object%20Reference) (OtherComp :type Primitive%20Component%20Object%20Reference) (OtherBodyIndex :type Integer))
  (Utilities|Casting|CastToBP_Santa OtherActor)
  (Variables|Default|SetinRange false)
  (Pawn|Components|CharacterMovement|SetMovementMode (Variables|Character|GetCharacterMovement) "MOVE_NavWalking" 0)
  (CallFunction|ChasePlayer))

(event Custom|Random%20Roam
  (if (not (Variables|Default|GetinRange))
    (Variables|/Script/Engine.CharacterMovementComponent|SetMaxWalkSpeed (Variables|Character|GetCharacterMovement) 1.5e+02)
    (AI|AIMoveTo self (.RandomLocation (AI|Navigation|GetRandomReachablePointinRadius (Transformation|GetActorLocation) 1e+03 0 0)) 0 5.0 false
      (:then
        (CallFunction|DecideNextAction)))))

(event Custom|DecideNextAction
  (Utilities|FlowControl|Delay (Math|Conversions|ToFloat(Integer) (Math|Random|RandomIntegerinRange 2 4)))
  (CallFunction|RandomRoam))

(event Custom|attacking
  (bind _tpc (Variables|Default|Gettpc))
  (if (Variables|Default|GetinRange)
    (Variables|Default|SetisAttacking true)
    (Utilities|FlowControl|Delay (Variables|Default|Getattackspeed))
    (Variables|/Game/ClausCrusadeContent/Blueprints/BP_Santa.BP_Santa_C|SetCurrent%20Health _tpc (- (Variables|/Game/ClausCrusadeContent/Blueprints/BP_Santa.BP_Santa_C|GetCurrent%20Health _tpc) (Variables|Default|Getdamage)))
    (Audio|PlaySound2D "/Game/ClausCrusadeContent/Blueprints/Arg/arg.arg" 1.0 1.0 0.0 0 0)
    (if (<= (Variables|/Game/ClausCrusadeContent/Blueprints/BP_Santa.BP_Santa_C|GetCurrent%20Health _tpc) 0.0)
      (Game|SetGamePaused true)
      (Class|LevelStreamingDynamic|LoadLevelInstancebySoftObjectPtr "/Game/ClausCrusadeContent/Levels/GameOver.GameOver" "0, 0, 0" "0, 0, 0" "" 0 false)
      (else
        (Variables|Default|SetisAttacking false)
        (CallFunction|ResetAttack)))
    (else
      (Variables|Default|SetisAttacking false)
      (CallFunction|ChasePlayer))))

(event Custom|Reset%20Attack
  (Utilities|FlowControl|DoOnce false) ; enters at Reset
)

(event Custom|Chase%20Player
  (bind _charactermovement (Variables|Character|GetCharacterMovement))
  (bind _asbp_santa (Utilities|Casting|CastToBP_Santa (Variables|Default|Gettarget))
    (:then
      (Variables|/Script/Engine.CharacterMovementComponent|SetMaxWalkSpeed _charactermovement 2.5e+02)
      (Pawn|Components|CharacterMovement|SetMovementMode _charactermovement "MOVE_NavWalking" 0)
      (AI|AIMoveTo self (Transformation|GetActorLocation _asbp_santa) 0 5e+01 false))
    (:CastFailed
      (Development|PrintString "Cast failed"))))

(event EventBeginPlay
  (CallFunction|RandomRoam))

(event EventTick
  (params (DeltaSeconds :type Float%20%28single-precision%29))
  (if (Variables|Default|GetinRange)
    (Utilities|FlowControl|Delay 1.0)
    (Utilities|FlowControl|DoOnce false
      (:Completed
        (CallFunction|Attacking)))
    (else
      (Utilities|FlowControl|Delay 1.0)
      (if (Variables|Default|Getfirstfind)
        (CallFunction|ChasePlayer)
        (else
          (CallFunction|DecideNextAction))))))

(event EventTakeDamage
  (params (Bone%20Name :type Name :default "None") (Damage :type Float%20%28double-precision%29))
  (bind _asbp_santa (Utilities|Casting|CastToBP_Santa (Variables|Default|Gettarget)))
  (if (== Bone%20Name "neck_01")
    (Variables|/Game/ClausCrusadeContent/Blueprints/BP_Santa.BP_Santa_C|Sethighscore _asbp_santa (+ (Variables|/Game/ClausCrusadeContent/Blueprints/BP_Santa.BP_Santa_C|Gethighscore _asbp_santa) 5))
    (Audio|PlaySound2D "/Game/ClausCrusadeContent/Blueprints/Arg/headshot.headshot" 1.0 1.0 0.0 0 0)
    (Variables|Default|SetHealth 0.0)
    (Variables|Default|SetisDead true)
    (Components|Movement|StopMovementImmediately (Variables|Character|GetCharacterMovement) :!label _label)
    (Class|SkeletalMeshComponent|SetAllBodiesSimulatePhysics (Variables|Character|GetMesh) true)
    (Collision|SetCollisionEnabled (Variables|Collision|GetCapsuleComponent) "NoCollision")
    (Utilities|FlowControl|Delay 5.0)
    (Actor|DestroyActor)
    (else
      (Variables|/Game/ClausCrusadeContent/Blueprints/BP_Santa.BP_Santa_C|Sethighscore _asbp_santa (+ (Variables|/Game/ClausCrusadeContent/Blueprints/BP_Santa.BP_Santa_C|Gethighscore _asbp_santa) 1))
      (bind _output_get (Variables|Default|SetHealth (- (Variables|Default|GetHealth) Damage)))
      (if (<= _output_get 0.0)
        (Variables|Default|SetisDead true)
        (goto _label)))))

(fn ConstructionScript)