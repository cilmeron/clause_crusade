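; DoDamageBP is a damage volume that drains BP_Santa's health while Santa stays inside its Box component.
; Begin overlap sets IsHit, then subtracts a fixed amount directly from CurrentHealth, repeating through a half-second Delay loop.
; End overlap by Santa clears IsHit, which stops the loop at its next check after the delay.
; Santa's validity is checked only before the first hit, and health is not clamped here.
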(event OnComponentBeginOverlap(Box)
  (params (OverlappedComponent :type Primitive%20Component%20Object%20Reference) (OtherActor :type Actor%20Object%20Reference) (OtherComp :type Primitive%20Component%20Object%20Reference) (OtherBodyIndex :type Integer) (bFromSweep :type Boolean) (SweepResult :type Hit%20Result%20Structure%20%28by%20ref%29))
  (bind _asbp_santa (Utilities|Casting|CastToBP_Santa OtherActor))
  (bind _output_get (Variables|Default|SetisHit true))
  (if _output_get
    (Utilities|IsValid _asbp_santa
      (:Is%20Valid
        (Variables|/Game/ClausCrusadeContent/Blueprints/BP_Santa.BP_Santa_C|SetCurrent%20Health _asbp_santa (- (Variables|/Game/ClausCrusadeContent/Blueprints/BP_Santa.BP_Santa_C|GetCurrent%20Health _asbp_santa) 5.0) :!label _label)
        (Utilities|FlowControl|Delay 0.5)
        (if (Variables|Default|GetisHit)
          (goto _label))))))

(event OnComponentEndOverlap(Box)
  (params (OverlappedComponent :type Primitive%20Component%20Object%20Reference) (OtherActor :type Actor%20Object%20Reference) (OtherComp :type Primitive%20Component%20Object%20Reference) (OtherBodyIndex :type Integer))
  (Utilities|Casting|CastToBP_Santa OtherActor)
  (Variables|Default|SetisHit false))

(event EventBeginPlay)

(event Collision|EventActorBeginOverlap
  (params (OtherActor :type Actor%20Object%20Reference)))

(event EventTick
  (params (DeltaSeconds :type Float%20%28single-precision%29)))

(fn ConstructionScript)