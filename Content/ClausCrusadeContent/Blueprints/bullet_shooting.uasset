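; Short-lived bullet projectile actor that applies damage and plays impact effects when its sphere hits something.
; On a hit, it line traces from the player camera to the impact point and sends a TakeDamage message with the hit bone name to the traced actor.
; It then plays a sound, spawns a small muzzle-flash emitter at that location, and destroys itself.
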(event OnComponentHit(Sphere)
  (params (HitComponent :type Primitive%20Component%20Object%20Reference) (OtherActor :type Actor%20Object%20Reference) (OtherComp :type Primitive%20Component%20Object%20Reference) (NormalImpulse :type Vector :default "0, 0, 0") (Hit :type Hit%20Result%20Structure%20%28by%20ref%29))
  (bind _outhit (Collision|LineTraceByChannel (Camera|GetCameraLocation (Game|GetPlayerCameraManager 0)) (.ImpactPoint (Collision|BreakHitResult Hit)) "TraceTypeQuery1" false 0 "None"))
  (Class|BPITakeDamage|TakeDamage(Message) (.HitActor (Collision|BreakHitResult _outhit)) (.HitBoneName (Collision|BreakHitResult _outhit)) 2e+01)
  (Audio|PlaySoundatLocation 0 (.Location (Collision|BreakHitResult _outhit)) "0, 0, 0" 1.0 1.0 0.0 0 0 0 0)
  (Effects|SpawnEmitteratLocation "/Game/InfinityBladeEffects/Effects/FX_Monsters/FX_Monster_Gruntling/Master/P_BackPack_MuzzleFlash.P_BackPack_MuzzleFlash" (.Location (Collision|BreakHitResult _outhit)) "0, 0, 0" "0.100000,0.100000,0.100000")
  (Actor|DestroyActor))

(event EventBeginPlay
  (Actor|SetLifeSpan 0.7))

(event Collision|EventActorBeginOverlap
  (params (OtherActor :type Actor%20Object%20Reference)))

(event EventTick
  (params (DeltaSeconds :type Float%20%28single-precision%29)))

(fn ConstructionScript)